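; Keyboard-controlled OpenManipulator robot arm Blueprint with four rotating joints, a two-finger gripper and a movable camera.
; Key presses and releases set direction states, which Tick turns into fixed per-frame local joint rotations and relative camera moves, without delta-time scaling.
; G plays and F reverses a timeline that slides the gripper links as mirror images.
; InitPose and HomePose are empty events, though key 1 and key 2 call them.
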(event `self.ReceivePossessed`
  (params (NewController :type "Controller Object Reference")))

(event `Init Pose`)

(event `Key|Y`
  (params (Key :type "Key Structure"))
  ;[1 1 1] Joint1
  (:`Pressed`
    (set `self.Joint1Rotate` 1))
  (:`Released`
    (set `self.Joint1Rotate` 0)))

(event `Key|U`
  (params (Key :type "Key Structure"))
  ;[1 1 1] Joint2
  (:`Pressed`
    (set `self.Joint2Rotate` 1))
  (:`Released`
    (set `self.Joint2Rotate` 0)))

(event `Key|I`
  (params (Key :type "Key Structure"))
  ;[1 1 1] Joint3
  (:`Pressed`
    (set `self.Joint3Rotate` 1))
  (:`Released`
    (set `self.Joint3Rotate` 0)))

(event `Key|O`
  (params (Key :type "Key Structure"))
  ;[1 1 1] Joint4
  (:`Pressed`
    (set `self.Joint4Rotate` 1))
  (:`Released`
    (set `self.Joint4Rotate` 0)))

(event `Key|One`
  (params (Key :type "Key Structure"))
  ;[1 1 1] Pose
  (:`Pressed`
    (`self.Init Pose`)))

(event `Home Pose`)

(event `Key|H`
  (params (Key :type "Key Structure"))
  ;[1 1 1] Joint1
  (:`Pressed`
    (set `self.Joint1Rotate` -1))
  (:`Released`
    (set `self.Joint1Rotate` 0)))

(event `Key|J`
  (params (Key :type "Key Structure"))
  ;[1 1 1] Joint2
  (:`Pressed`
    (set `self.Joint2Rotate` -1))
  (:`Released`
    (set `self.Joint2Rotate` 0)))

(event `Key|K`
  (params (Key :type "Key Structure"))
  ;[1 1 1] Joint3
  (:`Pressed`
    (set `self.Joint3Rotate` -1))
  (:`Released`
    (set `self.Joint3Rotate` 0)))

(event `Key|L`
  (params (Key :type "Key Structure"))
  ;[1 1 1] Joint4
  (:`Pressed`
    (set `self.Joint4Rotate` -1))
  (:`Released`
    (set `self.Joint4Rotate` 0)))

(event `Key|Two`
  (params (Key :type "Key Structure"))
  ;[1 1 1] Pose
  (:`Pressed`
    (`self.Home Pose`)))

(event `self.ReceiveTick`
  (params (DeltaSeconds :type "Float (single-precision)"))
  (bind _joint2 (`self.Joint2`))
  (bind _joint1 (`self.Joint1`))
  (bind _joint3 (`self.Joint3`))
  (bind _joint4 (`self.Joint4`))
  (bind _camera (`self.Camera`))
  (bind _camerax (`self.cameraX`))
  (bind _camera_2 (`self.Camera`))
  (bind _cameray (`self.cameraY`))
  ;[1 1 1] Joint
  (if (== (`self.Increase`) (`self.Joint1Rotate`))
    (`SceneComponent.K2_AddLocalRotation` _joint1 (struct :`Yaw` 1.0) false false))
  (if (== (`self.Decrease`) (`self.Joint1Rotate`))
    (`SceneComponent.K2_AddLocalRotation` _joint1 (struct :`Yaw` -1.0) false false))
  (if (== (`self.Increase`) (`self.Joint2Rotate`))
    (`SceneComponent.K2_AddLocalRotation` _joint2 (struct :`Pitch` 1.0) false false))
  (if (== (`self.Decrease`) (`self.Joint2Rotate`))
    (`SceneComponent.K2_AddLocalRotation` _joint2 (struct :`Pitch` -1.0) false false))
  (if (== (`self.Increase`) (`self.Joint3Rotate`))
    (`SceneComponent.K2_AddLocalRotation` _joint3 (struct :`Pitch` 1.0) false false))
  (if (== (`self.Decrease`) (`self.Joint3Rotate`))
    (`SceneComponent.K2_AddLocalRotation` _joint3 (struct :`Pitch` -1.0) false false))
  (if (== (`self.Increase`) (`self.Joint4Rotate`))
    (`SceneComponent.K2_AddLocalRotation` _joint4 (struct :`Pitch` 1.0) false false))
  (if (== (`self.Decrease`) (`self.Joint4Rotate`))
    (`SceneComponent.K2_AddLocalRotation` _joint4 (struct :`Pitch` -1.0) false false))
  ;[1 1 1] Camera
  (if (== 1 _camerax)
    (`SceneComponent.K2_AddRelativeLocation` _camera_2 (1.0 0.0 0.0) false false))
  (if (== -1 _camerax)
    (`SceneComponent.K2_AddRelativeLocation` _camera_2 (-1.0 0.0 0.0) false false))
  (if (== 1 _cameray)
    (`SceneComponent.K2_AddRelativeLocation` _camera (0.0 -1.0 0.0) false false))
  (if (== -1 _cameray)
    (`SceneComponent.K2_AddRelativeLocation` _camera (0.0 1.0 0.0) false false)))

(event `Key|G`
  (params (Key :type "Key Structure"))
  ;[1 1 1] Gripper
  (:`Pressed`
    (bind (_direction _open_close) (`Timeline|タイムライン` :!label _label)
      (:`Update`
        (`SceneComponent.K2_SetRelativeLocation` (`self.test_chain_link_grip_r`) _open_close false false)
        (`SceneComponent.K2_SetRelativeLocation` (`self.test_chain_link_grip_l`) (* _open_close (1.0 -1.0 1.0)) false false)))))

(event `Key|F`
  (params (Key :type "Key Structure"))
  ;[1 1 1] Gripper
  (:`Pressed`
    (goto _label :!via `Reverse`)))

(event `Key|W`
  (params (Key :type "Key Structure"))
  ;[1 1 1] Camera
  (:`Pressed`
    (set `self.cameraX` 1))
  (:`Released`
    (set `self.cameraX` 0)))

(event `Key|S`
  (params (Key :type "Key Structure"))
  ;[1 1 1] Camera
  (:`Pressed`
    (set `self.cameraX` -1))
  (:`Released`
    (set `self.cameraX` 0)))

(event `Key|A`
  (params (Key :type "Key Structure"))
  ;[1 1 1] Camera
  (:`Pressed`
    (set `self.cameraY` 1))
  (:`Released`
    (set `self.cameraY` 0)))

(event `Key|D`
  (params (Key :type "Key Structure"))
  ;[1 1 1] Camera
  (:`Pressed`
    (set `self.cameraY` -1))
  (:`Released`
    (set `self.cameraY` 0)))

(fn `UserConstructionScript`)